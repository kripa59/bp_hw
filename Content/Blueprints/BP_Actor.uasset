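; BP_Actor is an actor with two cube components, Cube and Cube1, and small functions that add fixed world rotations to them.
; Separate functions rotate each cube on a different axis, and NewFunction_0 wraps a call to RotateFirstCubeFunc.
; The event stubs are empty and the EventGraph rotation nodes are unconnected, leaving only a zero rotation of Cube1 in the construction script.
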(event EventBeginPlay)

(event Collision|EventActorBeginOverlap
  (params (OtherActor :type Actor%20Object%20Reference)))

(event EventTick
  (params (DeltaSeconds :type Float%20%28single-precision%29)))

(event Collision|EventHit
  (params (MyComp :type Primitive%20Component%20Object%20Reference) (Other :type Actor%20Object%20Reference) (OtherComp :type Primitive%20Component%20Object%20Reference) (bSelfMoved :type Boolean) (HitLocation :type Vector :default "0, 0, 0") (HitNormal :type Vector :default "0, 0, 0") (NormalImpulse :type Vector :default "0, 0, 0") (Hit :type Hit%20Result%20Structure%20%28by%20ref%29)))

(fn ConstructionScript
  (Transformation|AddWorldRotation (Variables|Default|GetCube1) "0, 0, 0" false false))

(fn RotateFirstCubeFunc
  (Transformation|AddWorldRotation (Variables|Default|GetCube) "77.000000, 0,0.000000" false false))

(fn RotateSecondCubeFunc
  (Transformation|AddWorldRotation (Variables|Default|GetCube1) "0.000000,6.000000,0.000000" false false))

(fn NewFunction0
  (CallFunction|RotateFirstCubeFunc))

(fn RotateFirstCubeFunc
  (Transformation|AddWorldRotation (Variables|Default|GetCube) "0, 0, 0" false false))